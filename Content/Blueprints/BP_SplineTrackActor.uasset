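; Track actor that builds a deformed mesh track along an editable spline, with an optional closed loop.
; The construction script adds one spline mesh component per spline point, using TrackPartMesh and bending it toward the next point with local positions and tangents.
; Each segment also takes its start and end roll and cross-section scale from the spline points, so banking and width follow the spline.
; All logic runs at construction, as the event graph is empty.
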(event EventBeginPlay)

(event Collision|EventActorBeginOverlap
  (params (OtherActor :type Actor%20Object%20Reference)))

(event EventTick
  (params (DeltaSeconds :type Float%20%28single-precision%29)))

(fn ConstructionScript
  (Spline|SetClosedLoop (Variables|Default|GetTrack_Spline) (Variables|Default|GetClosed%20Loop%20?) true)
  (for _index (range 0 (- (Spline|GetNumberOfSplinePoints (Variables|Default|GetTrack_Spline)) 1))
    (LocalVariables|SetStart%20Point _index)
    (LocalVariables|SetEnd%20Point (+ _index 1))
    (bind _returnvalue (AddComponent|AddSplineMeshComponent false))
    (bind _output_get (LocalVariables|SetCurrent%20Spline%20Mesh _returnvalue))
    (Components|StaticMesh|SetStaticMesh _output_get (Variables|Default|GetTrack%20Part%20Mesh))
    (SplineMesh|SetStartandEnd (LocalVariables|GetCurrent%20Spline%20Mesh) (.Location (Spline|GetLocationandTangentatSplinePoint (Variables|Default|GetTrack_Spline) _index "Local")) (.Tangent (Spline|GetLocationandTangentatSplinePoint (Variables|Default|GetTrack_Spline) _index "Local")) (.Location (Spline|GetLocationandTangentatSplinePoint (Variables|Default|GetTrack_Spline) (+ _index 1) "Local")) (.Tangent (Spline|GetLocationandTangentatSplinePoint (Variables|Default|GetTrack_Spline) (+ _index 1) "Local")) true :!class /Script/Engine.SplineMeshComponent)
    (Class|SplineMeshComponent|SetStartRoll (LocalVariables|GetCurrent%20Spline%20Mesh) (Math|Trig|DegreesToRadians (Spline|GetRollatSplinePoint (Variables|Default|GetTrack_Spline) (LocalVariables|GetStart%20Point) "Local")) true)
    (Class|SplineMeshComponent|SetEndRoll (LocalVariables|GetCurrent%20Spline%20Mesh) (Math|Trig|DegreesToRadians (Spline|GetRollatSplinePoint (Variables|Default|GetTrack_Spline) (LocalVariables|GetEnd%20Point) "Local")) true)
    (SplineMesh|SetStartScale (LocalVariables|GetCurrent%20Spline%20Mesh) (Math|Vector2D|MakeVector2D (.y (Spline|GetScaleatSplinePoint (Variables|Default|GetTrack_Spline) (LocalVariables|GetStart%20Point))) (.z (Spline|GetScaleatSplinePoint (Variables|Default|GetTrack_Spline) (LocalVariables|GetStart%20Point)))) true :!class /Script/Engine.SplineMeshComponent)
    (SplineMesh|SetEndScale (LocalVariables|GetCurrent%20Spline%20Mesh) (Math|Vector2D|MakeVector2D (.y (Spline|GetScaleatSplinePoint (Variables|Default|GetTrack_Spline) (LocalVariables|GetEnd%20Point))) (.z (Spline|GetScaleatSplinePoint (Variables|Default|GetTrack_Spline) (LocalVariables|GetEnd%20Point)))) true :!class /Script/Engine.SplineMeshComponent)))