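; CP_1 is a kart race checkpoint that counts laps and ends the race.
; When a BP_KartPawnPlayer overlaps its box with checkpoint index 0, it advances that kart's checkpoint and lap counters.
; When the lap counter reaches 4, compared as a string, FinishRace disables player 0's input, plays the finish sound and shows the WG_Finished_Race widget.
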(event OnComponentBeginOverlap(Box)
  (params (OverlappedComponent :type Primitive%20Component%20Object%20Reference) (OtherActor :type Actor%20Object%20Reference) (OtherComp :type Primitive%20Component%20Object%20Reference) (OtherBodyIndex :type Integer) (bFromSweep :type Boolean) (SweepResult :type Hit%20Result%20Structure%20%28by%20ref%29))
  (bind _asbp_kart_pawn_player (Utilities|Casting|CastToBP_KartPawnPlayer OtherActor))
  (if (== (Variables|/Game/Blueprints/BP_KartPawnPlayer.BP_KartPawnPlayer_C|GetCurren_Checkpoint _asbp_kart_pawn_player) 0)
    (Variables|/Game/Blueprints/BP_KartPawnPlayer.BP_KartPawnPlayer_C|SetCurren_Checkpoint _asbp_kart_pawn_player (+ (Variables|/Game/Blueprints/BP_KartPawnPlayer.BP_KartPawnPlayer_C|GetCurren_Checkpoint _asbp_kart_pawn_player) 1))
    (bind _output_get (Variables|/Game/Blueprints/BP_KartPawnPlayer.BP_KartPawnPlayer_C|SetCurrent_Lap _asbp_kart_pawn_player (+ (Variables|/Game/Blueprints/BP_KartPawnPlayer.BP_KartPawnPlayer_C|GetCurrent_Lap _asbp_kart_pawn_player) 1)))
    (if (Utilities|Enum|Equal(Enum) (Utilities|String|ToString(Integer) _output_get) "4")
      (CallFunction|FinishRace))))

(event Custom|Finish%20Race
  (Input|DisableInput (Game|Player|GetPlayerPawn 0) (Game|GetPlayerController 0))
  (Audio|PlaySound2D "/Game/Audio/Lap_Finish.Lap_Finish" 1.0 1.0 0.0 0 0)
  (bind _returnvalue (UserInterface|CreateWidget "/Game/Blueprints/WG_Finished_Race.WG_Finished_Race_C"))
  (UserInterface|Viewport|AddtoViewport _returnvalue 0))

(event EventBeginPlay)

(event Collision|EventActorBeginOverlap
  (params (OtherActor :type Actor%20Object%20Reference)))

(event EventTick
  (params (DeltaSeconds :type Float%20%28single-precision%29)))

(fn ConstructionScript)