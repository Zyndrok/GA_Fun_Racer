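; BP_Normal_Street is a spline-based street builder that lays TrackPartMesh along TrackSpline in the construction script, with no runtime logic.
; It optionally closes the loop, then adds spline mesh components at DefaultSpacing intervals, taking positions and tangents by distance along the spline.
; Roll and cross-section scale instead use the segment index as a spline point index, so they match only if points align with the spacing.
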(event EventBeginPlay)

(event Collision|EventActorBeginOverlap
  (params (OtherActor :type Actor%20Object%20Reference)))

(event EventTick
  (params (DeltaSeconds :type Float%20%28single-precision%29)))

(fn ConstructionScript
  (bind _track_spline (Variables|Default|GetTrack_Spline))
  (bind _track_spline_2 (Variables|Default|GetTrack_Spline))
  (Spline|SetClosedLoop (Variables|Default|GetTrack_Spline) (Variables|Default|GetClosed%20Loop%20?) true)
  (for _index (range 0 (Math|Float|Truncate (/ (Spline|GetSplineLength (Variables|Default|GetTrack_Spline)) (Variables|Default|GetDefault%20Spacing))))
    (LocalVariables|SetStart%20Point _index)
    (LocalVariables|SetEnd%20Point (+ _index 1))
    (bind _returnvalue (AddComponent|AddSplineMeshComponent false))
    (bind _output_get (LocalVariables|SetCurrent%20Spline%20Mesh _returnvalue))
    (Components|StaticMesh|SetStaticMesh _output_get (Variables|Default|GetTrack%20Part%20Mesh))
    (SplineMesh|SetStartandEnd (LocalVariables|GetCurrent%20Spline%20Mesh) (Spline|GetLocationatDistanceAlongSpline _track_spline_2 (* _index (Variables|Default|GetDefault%20Spacing)) "Local") (Spline|GetTangentatDistanceAlongSpline _track_spline_2 (* _index (Variables|Default|GetDefault%20Spacing)) "Local") (Spline|GetLocationatDistanceAlongSpline _track_spline (* (+ _index 1) (Variables|Default|GetDefault%20Spacing)) "Local") (Spline|GetTangentatDistanceAlongSpline _track_spline (* (+ _index 1) (Variables|Default|GetDefault%20Spacing)) "Local") true :!class /Script/Engine.SplineMeshComponent)
    (Class|SplineMeshComponent|SetStartRoll (LocalVariables|GetCurrent%20Spline%20Mesh) (Math|Trig|DegreesToRadians (Spline|GetRollatSplinePoint (Variables|Default|GetTrack_Spline) (LocalVariables|GetStart%20Point) "Local")) true)
    (Class|SplineMeshComponent|SetEndRoll (LocalVariables|GetCurrent%20Spline%20Mesh) (Math|Trig|DegreesToRadians (Spline|GetRollatSplinePoint (Variables|Default|GetTrack_Spline) (LocalVariables|GetEnd%20Point) "Local")) true)
    (SplineMesh|SetStartScale (LocalVariables|GetCurrent%20Spline%20Mesh) (Math|Vector2D|MakeVector2D (.y (Spline|GetScaleatSplinePoint (Variables|Default|GetTrack_Spline) (LocalVariables|GetStart%20Point))) (.z (Spline|GetScaleatSplinePoint (Variables|Default|GetTrack_Spline) (LocalVariables|GetStart%20Point)))) true :!class /Script/Engine.SplineMeshComponent)
    (SplineMesh|SetEndScale (LocalVariables|GetCurrent%20Spline%20Mesh) (Math|Vector2D|MakeVector2D (.y (Spline|GetScaleatSplinePoint (Variables|Default|GetTrack_Spline) (LocalVariables|GetEnd%20Point))) (.z (Spline|GetScaleatSplinePoint (Variables|Default|GetTrack_Spline) (LocalVariables|GetEnd%20Point)))) true :!class /Script/Engine.SplineMeshComponent)))