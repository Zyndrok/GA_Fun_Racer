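; Shisha coals trap actor that affects karts driving into it.
; When a BP_KartPawnBase overlaps its Box, it calls ActivateShishaTrap on that kart and destroys itself; other actors are ignored.
; The construction script traces downward and, on a hit, rotates the actor to the surface normal with a corrective local rotation, so placed coals follow the ground slope.
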(event OnComponentBeginOverlap(Box)
  (params (OverlappedComponent :type Primitive%20Component%20Object%20Reference) (OtherActor :type Actor%20Object%20Reference) (OtherComp :type Primitive%20Component%20Object%20Reference) (OtherBodyIndex :type Integer) (bFromSweep :type Boolean) (SweepResult :type Hit%20Result%20Structure%20%28by%20ref%29))
  (bind _asbp_kart_pawn_base (Utilities|Casting|CastToBP_KartPawnBase OtherActor))
  (Default|ActivateShishaTrap _asbp_kart_pawn_base)
  (Actor|DestroyActor))

(fn ConstructionScript
  (bind _returnvalue (Transformation|GetActorLocation))
  (bind (_outhit _returnvalue_2) (Collision|LineTraceByChannel _returnvalue (- _returnvalue "0, 0,400.000000") "TraceTypeQuery1" false 0 "None"))
  (if _returnvalue_2
    (Transformation|SetActorRotation (Math|Conversions|RotationFromXVector (.Normal (Collision|BreakHitResult _outhit))))
    (Transformation|AddActorLocalRotation "-90.000000, 0, 0" false false)))