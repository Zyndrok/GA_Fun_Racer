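; BP_PickUpBox is a pickup box that gives a random tool to any kart that overlaps it.
; It rolls one of three tool options on BeginPlay and passes it to the overlapping BP_KartPawnBase through LOCALSetCurrentTool.
; A pickup hides the cube and blocks further pickups for a cooldown, then reshows it and rerolls.
; A bob-and-spin timeline exists but is never started.
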(event OnComponentBeginOverlap(Box)
  (params (OverlappedComponent :type Primitive%20Component%20Object%20Reference) (OtherActor :type Actor%20Object%20Reference) (OtherComp :type Primitive%20Component%20Object%20Reference) (OtherBodyIndex :type Integer) (bFromSweep :type Boolean) (SweepResult :type Hit%20Result%20Structure%20%28by%20ref%29))
  (if (not (Variables|Default|GetbCooldown))
    (bind _asbp_kart_pawn_base (Utilities|Casting|CastToBP_KartPawnBase OtherActor))
    (Variables|Default|SetbCooldown true)
    (Rendering|SetVisibility (Variables|Default|GetCube) false true)
    (Default|LOCALSetCurrentTool _asbp_kart_pawn_base (Variables|Default|GetTool))
    (Utilities|FlowControl|Delay (Variables|Default|GetCooldownTime))
    (Variables|Default|SetbCooldown false)
    (Rendering|SetVisibility (Variables|Default|GetCube) true true)
    (CallFunction|RandomTool)))

(event Custom|RandomTool
  (Variables|Default|SetTool (Utilities|Select :Index (Math|Random|RandomIntegerinRange 0 2) :Option%200 "NewEnumerator0" :Option%201 "NewEnumerator1" :Option%202 "NewEnumerator2")))

(event EventBeginPlay
  (CallFunction|RandomTool))

(fn ConstructionScript)