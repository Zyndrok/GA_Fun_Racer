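; AI kart pawn that drives itself along a spline path taken from a path actor or set directly.
; While simulating physics on the ground, Tick feeds computed steering and throttle into the kart's inputs.
; Inputs come from dot products toward a speed-scaled look-ahead point on the spline, easing throttle in turns and turning slowly when facing away.
; Straying too far from the spline respawns the kart just above its closest point.
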(event Custom|Set%20Spline%20Path%20Actor
  (params (New%20Path%20Actor :type BP%20AI%20Spline%20Path%20Actor%20Object%20Reference))
  (bind _output_get (Variables|Default|SetPath%20Actor%20Reference New%20Path%20Actor))
  (Variables|Default|SetSpline%20Component%20Reference (Actor|GetComponentbyClass _output_get "/Script/Engine.SplineComponent")))

(event Custom|Set%20Path%20Spline%20Component
  (params (New%20Spline%20Component :type Spline%20Component%20Object%20Reference))
  (Variables|Default|SetSpline%20Component%20Reference New%20Spline%20Component))

(event EventBeginPlay
  (|CallParentFunction)
  (bind _path_actor_reference (Variables|Default|GetPath%20Actor%20Reference)
    (:then
      (Variables|Default|SetSpline%20Component%20Reference (Actor|GetComponentbyClass _path_actor_reference "/Script/Engine.SplineComponent")))
    (:else)))

(event EventTick
  (params (DeltaSeconds :type Float%20%28single-precision%29))
  (|CallParentFunction DeltaSeconds)
  (if (Physics|IsSimulatingPhysics (Variables|Default|GetKart_Collision) "None")
    (Variables|Default|GetPath%20Actor%20Reference
      (:then
        (if (Variables|Default|GetIs%20Moving%20On%20Ground?)
          (bind (_steering_axis _throttle_axis) (CallFunction|GetInputValues))
          (CallFunction|SetSteeringInput _steering_axis)
          (CallFunction|SetThrottleInput _throttle_axis)))
      (:else))))

(fn ConstructionScript
  (|CallParentFunction))

(fn GetInputValues
  (bind _returnvalue (Transformation|GetActorForwardVector))
  (bind _returnvalue_2 (Transformation|GetActorRightVector))
  (bind _returnvalue_3 (|GetDirectionToDestination))
  (bind _returnvalue_4 (|GetSteeringStrength(Between1.0&3.0)))
  (bind _spline_component_reference (Variables|Default|GetSpline%20Component%20Reference))
  (bind _returnvalue_5 (Math|Vector|DotProduct _returnvalue_3 _returnvalue_2))
  (bind _returnvalue_6 (Math|Vector|DotProduct _returnvalue_3 _returnvalue))
  (bind _returnvalue_7 (< _returnvalue_6 -0.2))
  (bind _returnvalue_8 (Math|Float|Absolute(Float) _returnvalue_5))
  (LocalVariables|SetCurrent%20Distance%20Offset (Math|Float|Max(Float) (Variables|Default|GetMin%20Distance%20Offset) (* (Variables|Default|GetCurrent%20Horizontal%20Speed) 0.9)))
  (LocalVariables|SetCurrent%20Closest%20Distance (|GetClosestDistanceToKartOnSpline))
  (LocalVariables|SetCurrent%20Destination%20On%20Path (stale _returnvalue))
  (Utilities|FlowControl|Sequence
    (:then_1
      (if (> (Math|Vector|VectorLength (- (Spline|GetLocationatDistanceAlongSpline _spline_component_reference (LocalVariables|GetCurrent%20Closest%20Distance) "World") (Transformation|GetActorLocation))) (Variables|Default|GetMin%20Off%20Track%20Distance))
        (CallFunction|OnRespawn (+ (Spline|GetLocationatDistanceAlongSpline _spline_component_reference (LocalVariables|GetCurrent%20Closest%20Distance) "World") (* (Math|Vector|GetUpVector (Spline|GetRotationatDistanceAlongSpline _spline_component_reference (LocalVariables|GetCurrent%20Closest%20Distance) "World")) (* (.SphereRadius (Collision|GetComponentBounds (Variables|Default|GetKart_Collision))) 2.0))) (Spline|GetRotationatDistanceAlongSpline _spline_component_reference (LocalVariables|GetCurrent%20Closest%20Distance) "World"))
        (return 0.0 0.0)))
    (:then_2
      (return (select _returnvalue_7 0.5 (select (< _returnvalue_8 (* _returnvalue_4 0.1)) 0.0 (* _returnvalue_4 _returnvalue_5 2.0))) (select _returnvalue_7 0.2 (Math|Float|Lerp (Math|Float|Absolute(Float) _returnvalue_6) 0.3 _returnvalue_8))))))